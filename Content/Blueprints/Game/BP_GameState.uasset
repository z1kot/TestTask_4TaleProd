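; BP_GameState is the Game State that runs a timed match and announces its start and end.
; StartGame stores the duration, starts a one-shot timer and multicasts the start, so remote machines run their own copy of the timer.
; EndGame acts only on authority, telling BP_GameMode to end the game before multicasting the end.
; Both multicasts fire event dispatchers for listeners on each machine.
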(event Custom|MC_GameStarted
  (params (Duration :type Float%20%28double-precision%29))
  (Default|CallOnGameStarted)
  (Networking|SwitchHasAuthority
    (:Remote
      (CallFunction|StartGameTimer Duration))))

(event Custom|MC_GameEnded
  (Default|CallOnGameEnded))

(fn ConstructionScript)

(fn StartGame
  (params (Duration :type Float%20%28single-precision%29))
  (Variables|Default|SetGameDuration Duration)
  (CallFunction|StartGameTimer (Variables|Default|GetGameDuration))
  (CallFunction|MCGameStarted (Variables|Default|GetGameDuration)))

(fn EndGame
  (Networking|SwitchHasAuthority
    (:Authority
      (bind _asbp_game_mode (Utilities|Casting|CastToBP_GameMode (Game|GetGameMode)))
      (Default|EndGame _asbp_game_mode)
      (CallFunction|MCGameEnded))))

(fn StartGameTimer
  (params (Duration :type Float%20%28double-precision%29))
  (bind _returnvalue (Utilities|Time|SetTimerbyEvent (EventDispatchers|CreateEvent :!event EndGame) Duration))
  (Variables|Default|SetGameTimer _returnvalue))