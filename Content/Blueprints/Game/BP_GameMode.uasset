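; Game mode that runs a timed match and handles player deaths and respawns.
; StartGame starts the BP_GameState timer if it is not already running and binds to each player state's death event.
; On death, it requests a delayed respawn from the player state and immediately teleports the pawn high above a random PlayerStart.
; EndGame disables input on every player's pawn.
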(event EventBeginPlay
  (bind _asbp_game_state (Utilities|Casting|CastToBP_GameState (Game|GetGameState)))
  (Variables|Default|SetMyGameState _asbp_game_state))

(fn ConstructionScript)

(fn StartGame
  (if (not (Utilities|Time|IsTimerActivebyHandle (Variables|/Game/Blueprints/Game/BP_GameState.BP_GameState_C|GetGameTimer (Variables|Default|GetMyGameState))))
    (Default|StartGame (Variables|Default|GetMyGameState) (Variables|Default|GetGameDuration))
    (for _array_element (Variables|/Script/Engine.GameStateBase|GetPlayerArray (Variables|Default|GetMyGameState))
      (bind _asbp_player_state (Utilities|Casting|CastToBP_PlayerState _array_element))
      (EventDispatchers|BindEventtoOnPlayerDead _asbp_player_state (EventDispatchers|CreateEvent :!event OnPlayerDead)))))

(fn EndGame
  (for _array_element (Variables|/Script/Engine.GameStateBase|GetPlayerArray (Variables|Default|GetMyGameState))
    (bind _asbp_player (Utilities|Casting|CastToBP_Player (PlayerState|GetPawn _array_element)))
    (Default|ToggleInput _asbp_player false)))

(fn OnPlayerDead
  (params (Player :type Player%20State%20Object%20Reference))
  (bind _asbp_player_state (Utilities|Casting|CastToBP_PlayerState Player))
  (Default|DelayedRespawnPlayer _asbp_player_state 2.0)
  (bind _outactors (Actor|GetAllActorsOfClass "/Script/Engine.PlayerStart"))
  (Transformation|SetActorLocationAndRotation (PlayerState|GetPawn Player) (+ "0.000000,0.000000,2500.000000" (Transformation|GetActorLocation (.OutItem (Utilities|Array|Random _outactors)))) "0, 0, 0" false true))