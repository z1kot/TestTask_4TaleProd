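; Player controller that adds the default Enhanced Input mapping context and handles toggling the inventory screen.
; On BeginPlay it caches the BP_HUD reference only on the non-authority (client) side.
; The inventory input action and CloseInventory event both call OpenInventory, a toggle that adds or removes the HUD's inventory widget.
; The toggle also switches pawn input, cursor visibility and input mode.
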(event Input|EnhancedActionEvents|EnhancedInputActionIA_Inventory
  (params (ActionValue :type Boolean) (ElapsedSeconds :type Float%20%28double-precision%29) (TriggeredSeconds :type Float%20%28double-precision%29) (InputAction :type Input%20Action%20Object%20Reference :default "/Game/Blueprints/Input/Actions/IA_Inventory.IA_Inventory"))
  ;[0 0.1912 1] Inventory
  (:Started
    (CallFunction|OpenInventory)))

(event EventCloseInventory
  ;[0 0.1912 1] Inventory
  (CallFunction|OpenInventory))

(event EventBeginPlay
  (bind _returnvalue (PlayerController|LocalPlayerSubsystems|GetEnhancedInputLocalPlayerSubsystem))
  (Utilities|FlowControl|Sequence
    (:then_0
      ;[0 0.1912 1] Save HUD ref only on client
      (Networking|SwitchHasAuthority
        (:Remote
          (bind _asbp_hud (Utilities|Casting|CastToBP_HUD (HUD|GetHUD)))
          (Variables|Default|SetHUD _asbp_hud))))
    (:then_1
      (Utilities|IsValid _returnvalue
        (:Is%20Valid
          (Input|AddMappingContext _returnvalue "/Game/Blueprints/Input/IMC_Default.IMC_Default" 0 "(bIgnoreAllPressedKeysUntilRelease=True,bForceImmediately=False,bNotifyUserSettings=False)"))))))

(fn ConstructionScript)

(fn OpenInventory
  (bind _returnvalue (Pawn|GetControlledPawn))
  (bind _hud (Variables|Default|GetHUD))
  (bind _inventory (Variables|/Game/Blueprints/Game/BP_HUD.BP_HUD_C|GetInventory _hud))
  (if (UserInterface|Viewport|IsinViewport (Variables|/Game/Blueprints/Game/BP_HUD.BP_HUD_C|GetInventory (Variables|Default|GetHUD)))
    (Widget|RemovefromParent _inventory)
    (Input|EnableInput _returnvalue 0)
    (Variables|Default|SetbShowMouseCursor false)
    (Input|SetInputModeGameOnly self false)
    (else
      (UserInterface|Viewport|AddtoViewport _inventory 0)
      (Input|DisableInput _returnvalue 0)
      (Variables|Default|SetbShowMouseCursor true)
      (Input|SetInputModeGameandUI self (Variables|/Game/Blueprints/Game/BP_HUD.BP_HUD_C|GetInventory (Variables|Default|GetHUD)) "DoNotLock" false false))))