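; BP_DamageZone is an area hazard that periodically damages every actor overlapping its Box component.
; The construction script sets the tick interval to DamageRate, so Tick serves as the repeating damage timer.
; Each tick branches on authority: the server applies Damage to all overlapping actors, while non-authoritative instances only reactivate the explosion particle.
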(event EventTick
  (params (DeltaSeconds :type Float%20%28single-precision%29))
  ;[0 0.1912 1] Tick(set by DamageRate)
  (Networking|SwitchHasAuthority
    (:Authority
      (CallFunction|DamageAll))
    (:Remote
      (CallFunction|PlayExplosionEffects))))

(fn ConstructionScript
  (Actor|Tick|SetActorTickInterval (Variables|Default|GetDamageRate)))

(fn DamageAll
  (for _array_element (Collision|GetOverlappingActors (Variables|Default|GetBox) "/Script/Engine.Actor" :!class /Script/Engine.PrimitiveComponent)
    (Game|Damage|ApplyDamage _array_element (Variables|Default|GetDamage) 0 self)))

(fn PlayExplosionEffects
  (Components|Activation|Activate (Variables|Default|GetExplosionParticle) true))