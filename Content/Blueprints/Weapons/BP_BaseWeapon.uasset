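; BP_BaseWeapon is a base weapon Blueprint that handles feedback for firing and reloading.
; Each of the two events first calls its dispatcher, OnWeaponUsed or OnWeaponReloading, on both authority and remote.
; Cosmetics then run only on the Remote branch of a Has Authority switch: muzzle particle and attached fire sound for shots, reload audio for reloads.
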(event EventOnWeaponFired
  (Default|CallOnWeaponUsed)
  (Networking|SwitchHasAuthority
    (:Remote
      (Components|Activation|Activate (Variables|Default|GetMuzzleParticle) true)
      (Audio|SpawnSoundAttached (Variables|Default|GetFireSound) (Variables|Transformation|GetRootComponent) "None" "0, 0, 0" "0, 0, 0" "KeepRelativeOffset" false 1.0 1.0 0.0 0 0))))

(event EventOnStartReloading
  (Default|CallOnWeaponReloading)
  (Networking|SwitchHasAuthority
    (:Remote
      (Components|Activation|Activate (Variables|Default|GetReloadAudio) true))))

(fn ConstructionScript)