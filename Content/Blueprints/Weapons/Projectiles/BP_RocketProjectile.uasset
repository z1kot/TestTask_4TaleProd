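; Rocket projectile that explodes on hit, dealing radial damage and knocking nearby objects away.
; CosmeticHit calls its parent, applies radial damage at the impact point, then runs RadialImpulse, a multi-sphere trace over the explosion radius.
; Impulses scale with Damage and target each hit actor's root primitive, or all its child components if the root isn't one.
; ApplyImpulse enables physics on Movable primitives that aren't yet simulating, so they get launched too.
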(event EventCosmeticHit
  (params (SweepResult :type Hit%20Result%20Structure%20%28by%20ref%29))
  (|CallParentFunction SweepResult)
  (Game|Damage|ApplyRadialDamage (Variables|Default|GetDamage) (.ImpactPoint (Collision|BreakHitResult SweepResult)) (Variables|Default|GetExplosionRadius) 0 0 self 0 false "ECC_Visibility")
  (CallFunction|RadialImpulse SweepResult))

(fn ConstructionScript)

(fn ApplyImpulse
  (params (TargetComp :type Scene%20Component%20Object%20Reference) (Impulse :type Vector))
  (bind _asprimitive_component (Utilities|Casting|CastToPrimitiveComponent TargetComp))
  (if (Physics|IsSimulatingPhysics _asprimitive_component "None")
    (Physics|AddImpulse _asprimitive_component Impulse "None" false :!label _label)
    (elif (Utilities|Enum|Equal(Enum) (Variables|/Script/Engine.SceneComponent|GetMobility _asprimitive_component) "Movable")
      (Physics|SetSimulatePhysics _asprimitive_component true)
      (goto _label))))

(fn RadialImpulse
  (params (Hit :type Hit%20Result%20Structure%20%28by%20ref%29))
  (bind _impactpoint (Collision|BreakHitResult Hit))
  (bind _outhits (Collision|MultiSphereTraceByChannel _impactpoint (+ _impactpoint "1.000000,-1.000000,0.500000") (Variables|Default|GetExplosionRadius) "TraceTypeQuery1" false 0 "None"))
  (for _array_element _outhits
    (if (Utilities|ClassIsChildOf (Utilities|GetClass (Variables|/Script/Engine.Actor|GetRootComponent (.HitActor (Collision|BreakHitResult _array_element)))) "/Script/Engine.PrimitiveComponent")
      (bind _output_get (LocalVariables|SetTargetScene (Variables|/Script/Engine.Actor|GetRootComponent (.HitActor (Collision|BreakHitResult _array_element)))))
      (CallFunction|ApplyImpulse _output_get (* (Math|Vector|Normalize (- (.ImpactPoint (Collision|BreakHitResult _array_element)) (Transformation|GetActorLocation))) (* (Variables|Default|GetDamage) 1e+02)) :!label _label)
      (else
        (for _array_element_2 (Components|GetChildrenComponents (Variables|/Script/Engine.Actor|GetRootComponent (.HitActor (Collision|BreakHitResult _array_element))) true)
          (LocalVariables|SetTargetScene _array_element_2)
          (goto _label))))))