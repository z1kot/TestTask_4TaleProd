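; Inventory component that holds a unique list of BaseItem actors and tracks one active item for its owner.
; S_-prefixed events forward use, stop-use and add requests to the matching functions.
; Added items take the owner, becoming active if none is, otherwise hiding; switching, directly or by index, hides the previous item and shows the new one attached.
; A RepNotify on ActiveItem broadcasts changes through OnActiveItem.
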(event Custom|S_StopUseActiveItem
  (CallFunction|StopUseActiveItem))

(event Custom|S_UseActiveItem
  (CallFunction|UseActiveItem))

(event Custom|S_AddToInventory
  (params (Item :type Actor%20Object%20Reference))
  (CallFunction|AddtoInventory Item))

(fn UseActiveItem
  (bind _activeitem (Variables|Default|GetActiveItem)
    (:then
      (Class|BaseItem|UseItem _activeitem))
    (:else)))

(fn StopUseActiveItem
  (bind _activeitem (Variables|Default|GetActiveItem)
    (:then
      (Class|BaseItem|StopUseItem _activeitem))
    (:else)))

(fn AddtoInventory
  (params (Item :type Actor%20Object%20Reference))
  (bind _asbase_item (Utilities|Casting|CastToBaseItem Item))
  (bind _returnvalue (Utilities|Array|AddUnique (Variables|Default|GetItems) _asbase_item))
  (if (CallFunction|NotIndexNone _returnvalue)
    (Actor|SetOwner Item (Components|GetOwner))
    (Variables|Default|GetActiveItem
      (:then
        (Class|BaseItem|HideandAttach _asbase_item))
      (:else
        (CallFunction|SetActiveItem _asbase_item)))))

(fn SetActiveItem
  (params (Item :type Base%20Item%20Object%20Reference))
  (Utilities|IsValid Item
    (:Is%20Valid
      (if (!= (Variables|Default|GetActiveItem) Item)
        (bind _activeitem (Variables|Default|GetActiveItem)
          (:then
            (Class|BaseItem|HideandAttach _activeitem))
          (:else
            _))
        (Variables|Default|SetActiveItem Item)
        (Class|BaseItem|ShowandAttach (Variables|Default|GetActiveItem) (Variables|Default|GetParrentAttachComp))))))

(fn SetActiveItembyIndex
  (params (ItemIndex :type Integer))
  (if (Utilities|Array|IsValidIndex (Variables|Default|GetItems) ItemIndex)
    (CallFunction|SetActiveItem (Utilities|Array|Get(acopy) (Variables|Default|GetItems) ItemIndex))))

(fn OnRepActiveItem
  (Default|CallOnActiveItem (Variables|Default|GetActiveItem)))